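; Player camera pawn with axis-driven planar movement, stepped mouse-wheel zoom on a spring arm, and a resource HUD.
; Holding the right mouse button hides the cursor and opens gates letting the mouse yaw the pawn and pitch the camera within limits.
; BeginPlay creates the HUD and stores floor extents, which movement never uses.
; Tick writes hardcoded placeholder meat and water values to the HUD.
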(event `self.ReceiveBeginPlay`
  ;[1 1 1] SET WORLD BOUNDS
  (`|ExecutionSequence`
    (:`then_0`
      (set `self.maxDistanceX` (.x (`.BoxExtent` (`self.GetActorBounds` (`|ConvertAsset` (`self.Floor`)) false)))))
    (:`then_1`
      (set `self.maxDistanceY` (.y (`.BoxExtent` (`self.GetActorBounds` (`|ConvertAsset` (`self.Floor`)) false)))))
    (:`then_2`
      (bind _returnvalue (`|CreateWidget` "/Game/Blueprints/HUD.HUD_C"))
      (bind _output_get (set `self.HUD Reference` _returnvalue))
      (`UserWidget.AddToViewport` _output_get 0))))

(event `self.ReceiveTick`
  (params (DeltaSeconds :type "Float (single-precision)"))
  (bind _hud_reference (`self.HUD Reference`))
  ;[1 1 1] Set Resource Variables
  (bind _output_get (set `/Game/Blueprints/HUD.meatValue` 15 _hud_reference))
  (`TextBlock.SetText` (`/Game/Blueprints/HUD.MeatShown` _hud_reference) (`KismetTextLibrary.Conv_IntToText` _output_get))
  (bind _output_get_2 (set `/Game/Blueprints/HUD.waterValue` 30 _hud_reference))
  (`TextBlock.SetText` (`/Game/Blueprints/HUD.WaterShown` _hud_reference) (`KismetTextLibrary.Conv_IntToText` _output_get_2)))

(event `InputAxis|MoveForward`
  (params (AxisValue :type "Float (single-precision)"))
  ;[1 1 1] MOVE FORWARD AND BACKWARD
  (`self.K2_AddActorLocalOffset` (`KismetMathLibrary.MakeVector` (* AxisValue (`self.MoveSpeed`)))))

(event `Key|MouseScrollUp`
  (params (Key :type "Key Structure" :default "AnyKey"))
  (bind _zoomspeed (`self.ZoomSpeed`))
  (bind _springarm (`self.SpringArm`))
  (bind _targetarmlength (`SpringArmComponent.TargetArmLength` _springarm))
  ;[1 1 1] ZOOM
  (:`Pressed`
    (if (> _targetarmlength (* _zoomspeed 3.0))
      (set `SpringArmComponent.TargetArmLength` (- _targetarmlength _zoomspeed) _springarm))))

(event `Key|MouseScrollDown`
  (params (Key :type "Key Structure" :default "AnyKey"))
  (bind _springarm (`self.SpringArm`))
  (bind _zoomspeed (`self.ZoomSpeed`))
  (bind _targetarmlength (`SpringArmComponent.TargetArmLength` _springarm))
  ;[1 1 1] ZOOM
  (:`Pressed`
    (if (< _targetarmlength (* _zoomspeed 40.0))
      (set `SpringArmComponent.TargetArmLength` (+ _zoomspeed _targetarmlength) _springarm))))

(event `InputAxis|MoveRight`
  (params (AxisValue :type "Float (single-precision)"))
  ;[1 1 1] MOVE LEFT AND RIGHT
  (`self.K2_AddActorLocalOffset` (`KismetMathLibrary.MakeVector` 0.0 (* AxisValue (`self.MoveSpeed`)))))

(event `InputAxisKey|MouseX`
  (params (AxisValue :type "Float (single-precision)"))
  ;[1 1 1] ROTATE
  (`/Engine/EditorBlueprintResources/StandardMacros.Gate` true :!label _label
    (:`Exit`
      (`self.K2_AddActorLocalRotation` (`KismetMathLibrary.MakeRotator` 0.0 0.0 (* (`self.RotateSpeed`) AxisValue))))))

(event `Key|RightMouseButton`
  (params (Key :type "Key Structure" :default "AnyKey"))
  (bind (_returnvalue_roll _returnvalue_pitch _returnvalue_yaw) (`KismetMathLibrary.BreakRotator` (`SceneComponent.K2_GetComponentRotation` (`self.Camera`))))
  ;[1 1 1] ROTATE
  (:`Pressed`
    (set `PlayerController.bShowMouseCursor` false (`GameplayStatics.GetPlayerController` 0))
    (`|ExecutionSequence`
      (:`then_0`
        (goto _label :!via `Open`))
      (:`then_1`
        (goto _label_2 :!via `Open`))))
  (:`Released`
    (set `PlayerController.bShowMouseCursor` true (`GameplayStatics.GetPlayerController` 0))
    (`|ExecutionSequence`
      (:`then_0`
        (goto _label :!via `Close`))
      (:`then_1`
        (goto _label_2 :!via `Close`)))))

(event `InputAxisKey|MouseY`
  (params (AxisValue :type "Float (single-precision)"))
  (bind (_returnvalue_roll _returnvalue_pitch _returnvalue_yaw) (`KismetMathLibrary.BreakRotator` (`SceneComponent.K2_GetComponentRotation` (`self.Camera`))))
  ;[1 1 1] ROTATE
  (`/Engine/EditorBlueprintResources/StandardMacros.Gate` true :!label _label_2
    (:`Exit`
      (`SceneComponent.K2_SetWorldRotation` (`self.Camera`) (`KismetMathLibrary.MakeRotator` _returnvalue_roll (`KismetMathLibrary.FClamp` (+ _returnvalue_pitch (* AxisValue (`self.RotateSpeed`))) -85.0 0.0) _returnvalue_yaw) false false))))

(fn `UserConstructionScript`)